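; BP_AutoDoor is a player-interactable swinging door that cycles through closed, partially open and open states, with optional auto-close when the player leaves its box.
; Tick polls the player's interact flag and hit actor, picking the swing side from a facing dot product and playing a state sound.
; HandleDoor interpolates yaw while interaction continues, and a timer advances the state.
; Auto-close rotates the door in one delayed call and resets the state on next interaction.
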(event `self.ReceiveBeginPlay`
  ;[0 0.6157 0.6118 0.502] Player Ref
  (bind _asbp_third_person_character (cast `/Game/DoorSystem/Player/Blueprints/BP_ThirdPersonCharacter` (`GameplayStatics.GetPlayerCharacter` 0)))
  (set `self.Player Ref` _asbp_third_person_character))

(event `HandleRotation`
  (params (SetRotation :type "Float (double-precision)"))
  ;[0 0.6157 0.6118 0.502] HandleRotation
  (`SceneComponent.K2_SetRelativeRotation` (`self.Door`) (`KismetMathLibrary.MakeRotator` 0.0 0.0 (`KismetMathLibrary.FInterpTo` (.yaw (`SceneComponent.RelativeRotation` (`self.Door`))) SetRotation (`GameplayStatics.GetWorldDeltaSeconds`) (`self.Interp Speed`))) false false))

(event `self.Box.OnComponentEndOverlap`
  (params (OverlappedComponent :type "PrimitiveComponent Object Reference") (OtherActor :type "Actor Object Reference") (OtherComp :type "PrimitiveComponent Object Reference") (OtherBodyIndex :type Integer))
  (bind _returnvalue (`GameplayStatics.GetPlayerCharacter` 0))
  (bind (_returnvalue_x _returnvalue_y) (`KismetMathLibrary.BreakVector` (`self.GetActorForwardVector` _returnvalue)))
  ;[0 0.6157 0.6118 0.502] AutoClose Door After Player Leave Collision Box
  (if (and (`self.AutoClose?`) (`self.DoorOpen?`))
    (if (and (== OtherActor _returnvalue) (or (>= _returnvalue_x _returnvalue_y) (<= _returnvalue_y _returnvalue_x)))
      (`KismetSystemLibrary.Delay` 0.2)
      (`self.AutoCloseDoor`)
      (set `self.AutoDoorActivated` true))))

(event `HandleDoor`
  ;[0 0.6157 0.6118 0.502] Handle Door ( Switch E num Based on Current State an Rotation )
  (switch `/Game/DoorSystem/Blueprints/Doors/Enumeration/E_DoorStates` (`self.EDoorStates`)
    (:`NewEnumerator0`
      (`self.HandleRotation` (* 15.0 (`self.Door Open Side`)))
      (set `self.DoorOpen?` true))
    (:`NewEnumerator1`
      (`self.HandleRotation` (* (`self.Door Open Angle`) (`self.Door Open Side`)))
      (set `self.DoorOpen?` true))
    (:`NewEnumerator2`
      (if (== (`self.Door Open Side`) 1.0)
        (`self.HandleRotation` -5.0)
        (else
          (`self.HandleRotation` 5.0)))
      (set `self.DoorOpen?` false))))

(event `AutoCloseDoor`
  ;[0 0.6157 0.6118 0.502] Auto Close Door Functionality
  ;;[0 0.6157 0.6118 0.502] Add Sound
  (`GameplayStatics.PlaySoundAtLocation` null (`self.K2_GetActorLocation`) (struct) 1.0 1.0 0.0 null null null null)
  (`SceneComponent.K2_SetRelativeRotation` (`self.Door`) (`KismetMathLibrary.MakeRotator` 0.0 0.0 (`KismetMathLibrary.FInterpTo` (.yaw (`SceneComponent.RelativeRotation` (`self.Door`))) 0.0 3.0 (`self.Interp Speed`))) false false))

(event `DoorSoundStates`
  (bind _returnvalue (`self.K2_GetActorLocation`))
  ;[0 0.6157 0.6118 0.502] Door Sounds Based On E_DoorStates
  (switch `/Game/DoorSystem/Blueprints/Doors/Enumeration/E_DoorStates` (`self.EDoorStates`)
    (:`NewEnumerator0`
      ;;[0 0.6157 0.6118 0.502] Add Sound
      (`GameplayStatics.PlaySoundAtLocation` null _returnvalue (struct) 1.0 1.0 0.0 null null null null))
    (:`NewEnumerator1`
      (`GameplayStatics.PlaySoundAtLocation` null _returnvalue (struct) 1.0 1.0 0.0 null null null null))
    (:`NewEnumerator2`
      (`GameplayStatics.PlaySoundAtLocation` null _returnvalue (struct) 1.0 1.0 0.0 null null null null))))

(event `IsInteractingWithDoor`
  (params (`Player Ref` :type "/Game/DoorSystem/Player/Blueprints/BP_ThirdPersonCharacter Object Reference"))
  ;[0 0.6157 0.6118 0.502] Door Interacting System
  (if (`self.AutoDoorActivated`)
    (set `self.EDoorStates` "NewEnumerator0")
    (set `self.AutoDoorActivated` false))
  (`self.DoorSoundStates`)
  (if (> (`KismetMathLibrary.Dot_VectorVector` (`self.GetActorForwardVector` `Player Ref`) (`SceneComponent.GetForwardVector` (`self.DoorOpenLocation`))) 0.0)
    (set `self.Door Open Side` 1.0)
    (else
      (set `self.Door Open Side` -1.0)))
  (set `self.bIsInteractingDoor?` true)
  (`KismetSystemLibrary.K2_SetTimerDelegate` (delegate `Stop Interacting`) (`self.Door Sound Time`)))

(event `Stop Interacting`
  ;[0 0.6157 0.6118 0.502] Door Interacting System
  (set `self.bIsInteractingDoor?` false)
  (switch `/Game/DoorSystem/Blueprints/Doors/Enumeration/E_DoorStates` (`self.EDoorStates`)
    (:`NewEnumerator0`
      (set `self.EDoorStates` "NewEnumerator1"))
    (:`NewEnumerator1`
      (set `self.EDoorStates` "NewEnumerator2"))
    (:`NewEnumerator2`
      (set `self.EDoorStates` "NewEnumerator0"))))

(event `self.ReceiveTick`
  (params (DeltaSeconds :type "Float (single-precision)"))
  (bind _player_ref (`self.Player Ref`))
  ;[0 0.6157 0.6118 0.502] Door Interaction
  (if (and (`/Game/DoorSystem/Player/Blueprints/BP_ThirdPersonCharacter.IsInteracting?` _player_ref) (== (`/Game/DoorSystem/Player/Blueprints/BP_ThirdPersonCharacter.HitActor` _player_ref) self))
    (if (`self.bIsInteractingDoor?`)
      (`self.HandleDoor`)
      (else
        (`self.IsInteractingWithDoor` (`self.Player Ref`))))))

(fn `UserConstructionScript`)